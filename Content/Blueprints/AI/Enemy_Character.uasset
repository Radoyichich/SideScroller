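; Enemy AI character that catches the player and can grab and climb ledges.
; Overlapping KillingBox flags the player as caught, snaps them in front of the enemy and raises the KillPlayer blackboard key for five seconds.
; HangingCheck uses forward and height sphere traces to snap the falling enemy onto a ledge in Flying mode.
; ClimbingLedge plays the climb montage, and UpdateWalkSpeed sets movement speed.
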(event OnComponentBeginOverlap(KillingBox)
  (params (OverlappedComponent :type Primitive%20Component%20Object%20Reference) (OtherActor :type Actor%20Object%20Reference) (OtherComp :type Primitive%20Component%20Object%20Reference) (OtherBodyIndex :type Integer) (bFromSweep :type Boolean) (SweepResult :type Hit%20Result%20Structure%20%28by%20ref%29))
  (bind _asthird_person_character (Utilities|Casting|CastToThirdPersonCharacter OtherActor))
  (if (not (Variables|/Game/Blueprints/Character/ThirdPersonCharacter.ThirdPersonCharacter_C|GetCaughtByEnemy _asthird_person_character))
    (AI|Components|Blackboard|SetValueasBool (AI|GetBlackboard 0) (Variables|Default|GetKillPlayer) true)
    (Variables|/Game/Blueprints/Character/ThirdPersonCharacter.ThirdPersonCharacter_C|SetCaughtByEnemy _asthird_person_character true)
    (Transformation|SetActorRotation _asthird_person_character (Transformation|GetActorRotation))
    (Transformation|SetActorLocation _asthird_person_character (+ (Transformation|GetActorLocation) (* (Transformation|GetActorForwardVector) 1e+01)) false false)
    (Utilities|FlowControl|Delay 5.0)
    (AI|Components|Blackboard|SetValueasBool (AI|GetBlackboard 0) (Variables|Default|GetKillPlayer) false)))

(fn ConstructionScript)

(fn UpdateWalkSpeed
  (params (New%20Walk%20Speed :type Float%20%28single-precision%29))
  (Variables|/Script/Engine.CharacterMovementComponent|SetMaxWalkSpeed (Variables|Character|GetCharacterMovement) New%20Walk%20Speed))