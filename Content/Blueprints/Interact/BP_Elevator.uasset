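; BP_Elevator is an interactable elevator that raises its mesh on Activate and returns it on Deactivate.
; Activate plays a timeline that lerps from the current location toward a point slightly above it each update, so the rise accumulates rather than targeting a fixed height.
; Deactivate plays a second timeline that lerps from the current location back to the position cached at BeginPlay.
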(event EventActivate
  (params (Character :type Character%20Object%20Reference))
  (bind _elevatormesh (Variables|Default|GetElevatorMesh))
  (bind _returnvalue (Transformation|GetWorldLocation _elevatormesh))
  (bind (_x _y _z) (Math|Vector|BreakVector _returnvalue))
  (bind _alpha (Timeline|Open_TL PlayFromStart)
    (:Update
      (Transformation|SetWorldLocation _elevatormesh (Math|Vector|Lerp(Vector) _returnvalue (Math|Vector|MakeVector _x _y (- _z -14.5)) _alpha) false false))))

(event EventDeactivate
  (params (Character :type Character%20Object%20Reference))
  (bind _elevatormesh (Variables|Default|GetElevatorMesh))
  (bind _alpha (Timeline|Close_TL PlayFromStart)
    (:Update
      (Transformation|SetWorldLocation _elevatormesh (Math|Vector|Lerp(Vector) (Transformation|GetWorldLocation _elevatormesh) (Variables|Default|GetInitialLocation) _alpha) false false))))

(event EventBeginPlay
  (Variables|Default|SetInitialLocation (Transformation|GetWorldLocation (Variables|Default|GetElevatorMesh))))

(fn ConstructionScript)