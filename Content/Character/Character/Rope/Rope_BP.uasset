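; Physics rope actor that lets the third-person character grab on, swing, climb and launch off, ticking only while the character is inside its trigger.
; Hold snaps the player to the nearest bone with mass, found via per-bone construction-script boxes, and passes on their incoming velocity.
; Tick ramps swing force, steps the active bone during climb montages, and keeps the capsule attached and rope-aligned.
; Unhold launches the player at double bone velocity.
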(event OnComponentBeginOverlap(TickTrigger)
  (params (OverlappedComponent :type Primitive%20Component%20Object%20Reference) (OtherActor :type Actor%20Object%20Reference) (OtherComp :type Primitive%20Component%20Object%20Reference) (OtherBodyIndex :type Integer) (bFromSweep :type Boolean) (SweepResult :type Hit%20Result%20Structure%20%28by%20ref%29))
  (Utilities|Casting|CastToThirdPersonCharacter OtherActor)
  (Actor|Tick|SetActorTickEnabled true))

(event OnComponentEndOverlap(TickTrigger)
  (params (OverlappedComponent :type Primitive%20Component%20Object%20Reference) (OtherActor :type Actor%20Object%20Reference) (OtherComp :type Primitive%20Component%20Object%20Reference) (OtherBodyIndex :type Integer))
  (Utilities|Casting|CastToThirdPersonCharacter OtherActor)
  (Actor|Tick|SetActorTickEnabled false))

(event EventBeginPlay
  (Actor|Tick|SetActorTickEnabled false))

(event Collision|EventActorBeginOverlap
  (params (OtherActor :type Actor%20Object%20Reference)))

(event EventHold
  (params (Character :type Character%20Object%20Reference))
  (bind _asthird_person_character (Utilities|Casting|CastToThirdPersonCharacter Character))
  (Variables|Default|SetPlayer _asthird_person_character)
  (Utilities|FlowControl|Sequence
    (:then_0
      ;[1 1 1] Get Rope Bone
      (bind _bestindex (CallFunction|FindNearestRopeBone))
      (Variables|Default|SetActiveBone (Class|SkinnedMeshComponent|GetBoneName (Variables|Default|GetRopeMesh) _bestindex)))
    (:then_1
      ;[1 1 1] Set Player Location And Movement
      (Transformation|SetWorldLocation (Variables|/Script/Engine.Character|GetCapsuleComponent (Variables|Default|GetPlayer)) (Transformation|GetSocketLocation (Variables|Default|GetRopeMesh) (Variables|Default|GetActiveBone)) false false)
      (Components|Movement|StopMovementImmediately (Variables|/Script/Engine.Character|GetCharacterMovement (Variables|Default|GetPlayer)))
      (Pawn|Components|CharacterMovement|SetMovementMode (Variables|/Script/Engine.Character|GetCharacterMovement (Variables|Default|GetPlayer)) "MOVE_Flying" 0)
      (Variables|/Game/Character/Character/ThirdPersonCharacter.ThirdPersonCharacter_C|SetIsOnRope (Variables|Default|GetPlayer) true)
      (Physics|SetPhysicsLinearVelocity (Variables|Default|GetRopeMesh) (Variables|Default|GetFirstVelocity) false (Variables|Default|GetActiveBone)))))

(event EventUnhold
  (params (Character :type Character%20Object%20Reference))
  (bind _asthird_person_character (Utilities|Casting|CastToThirdPersonCharacter Character))
  (bind _output_get (Variables|Default|SetPlayer _asthird_person_character))
  (Variables|/Game/Character/Character/ThirdPersonCharacter.ThirdPersonCharacter_C|SetIsOnRope _output_get false)
  (Pawn|Components|CharacterMovement|SetMovementMode (Variables|/Script/Engine.Character|GetCharacterMovement _output_get) "MOVE_Walking" 0)
  (Transformation|SetActorRotation (Variables|Default|GetPlayer) (Math|Rotator|MakeRotator 0.0 0.0 (.yaw (Transformation|GetActorRotation (Variables|Default|GetPlayer)))))
  (bind _returnvalue (Physics|GetPhysicsLinearVelocity (Variables|Default|GetRopeMesh) (Variables|Default|GetActiveBone)))
  (Character|LaunchCharacter (Variables|Default|GetPlayer) (* _returnvalue 2.0) true true))

(event EventTick
  (params (DeltaSeconds :type Float%20%28single-precision%29))
  (bind _asthird_person_character (Utilities|Casting|CastToThirdPersonCharacter (Game|GetPlayerCharacter 0)))
  (bind _output_get (Variables|Default|SetPlayer _asthird_person_character))
  (if (Variables|/Game/Character/Character/ThirdPersonCharacter.ThirdPersonCharacter_C|GetIsOnRope _output_get)
    (Utilities|FlowControl|Sequence
      (:then_0
        ;[1 1 1] Set Force
        (if (or (!= (Variables|/Game/Character/Character/ThirdPersonCharacter.ThirdPersonCharacter_C|GetForwardMove (Variables|Default|GetPlayer)) 0.0) (!= (Variables|/Game/Character/Character/ThirdPersonCharacter.ThirdPersonCharacter_C|GetRightMove (Variables|Default|GetPlayer)) 0.0))
          (Variables|Default|SetSwingForce (Math|Float|Clamp(Float) (+ (Variables|Default|GetSwingForce) 5e+01) 0.0 2e+03))
          (else
            (Variables|Default|SetSwingForce 0.0))))
      (:then_1
        ;[1 1 1] Climb Up/Down the Rope
        (if (not (Variables|Default|GetCharacterIsClimbing))
          (if (!= (Variables|/Game/Character/Character/ThirdPersonCharacter.ThirdPersonCharacter_C|GetForwardMove (Variables|Default|GetPlayer)) 0.0)
            (Utilities|FlowControl|DoOnce false :!label _label
              (:Completed
                (Physics|SetPhysicsLinearVelocity (Variables|Default|GetRopeMesh) "0, 0, 0" false "Bone_007")
                (Variables|Default|SetCharacterIsClimbing true)
                (bind _returnvalue (Animation|PlayAnimMontage (Variables|Default|GetPlayer) "/Game/Character/Animations/ClimbingARope4UE4_Montage.ClimbingARope4UE4_Montage" 2.0 "None"))
                (Variables|Default|SetActiveBone (Class|SkinnedMeshComponent|GetBoneName (Variables|Default|GetRopeMesh) (Math|Integer|Clamp(Integer) (+ (Class|SkinnedMeshComponent|GetBoneIndex (Variables|Default|GetRopeMesh) (Variables|Default|GetActiveBone)) (Math|Float|Truncate (* (Variables|/Game/Character/Character/ThirdPersonCharacter.ThirdPersonCharacter_C|GetForwardMove (Variables|Default|GetPlayer)) -7.0))) 38 94)))
                (Utilities|FlowControl|Delay (/ _returnvalue 2.0))
                (Variables|Default|SetCharacterIsClimbing false)
                (goto _label Reset))))))
      (:then_2
        ;[1 1 1] Swing Left/Right
        (if (!= (Variables|/Game/Character/Character/ThirdPersonCharacter.ThirdPersonCharacter_C|GetRightMove (Variables|Default|GetPlayer)) 0.0)
          (if (> (.Y (Math|Vector|BreakVector (Transformation|GetActorForwardVector (Variables|Default|GetPlayer)))) 0.0)
            (Physics|AddForce (Variables|Default|GetRopeMesh) (+ (* (Transformation|GetActorForwardVector (Variables|Default|GetPlayer)) (Variables|Default|GetSwingForce)) (Variables|/Game/Character/Character/ThirdPersonCharacter.ThirdPersonCharacter_C|GetRightMove (Variables|Default|GetPlayer))) (Variables|Default|GetActiveBone) true)
            (else
              (Physics|AddForce (Variables|Default|GetRopeMesh) (* (+ (* (Transformation|GetActorForwardVector (Variables|Default|GetPlayer)) (Variables|Default|GetSwingForce)) (Variables|/Game/Character/Character/ThirdPersonCharacter.ThirdPersonCharacter_C|GetRightMove (Variables|Default|GetPlayer))) -1.0) (Variables|Default|GetActiveBone) true)))))
      (:then_3
        ;[1 1 1] Set Player Location While On Rope
        (if (not (Variables|Default|GetCharacterIsClimbing))
          (Transformation|SetWorldLocation (Variables|/Script/Engine.Character|GetCapsuleComponent (Variables|Default|GetPlayer)) (Transformation|GetSocketLocation (Variables|Default|GetRopeMesh) (Variables|Default|GetActiveBone)) false true)
          (else
            (Components|MoveComponentTo (Variables|/Script/Engine.Character|GetCapsuleComponent (Variables|Default|GetPlayer)) (Transformation|GetSocketLocation (Variables|Default|GetRopeMesh) (Variables|Default|GetActiveBone)) (Math|Rotator|MakeRotator (.roll (Math|Rotator|MakeRotfromZY (- (Transformation|GetSocketLocation (Variables|Default|GetRopeMesh) "Bone_100") (Transformation|GetActorLocation (Variables|Default|GetPlayer))) (Math|Vector|Normalize (Math|Vector|CrossProduct (- (Transformation|GetSocketLocation (Variables|Default|GetRopeMesh) "Bone_100") (Transformation|GetActorLocation (Variables|Default|GetPlayer))) (Transformation|GetActorForwardVector (Variables|Default|GetPlayer)))))) (.pitch (Math|Rotator|MakeRotfromZY (- (Transformation|GetSocketLocation (Variables|Default|GetRopeMesh) "Bone_100") (Transformation|GetActorLocation (Variables|Default|GetPlayer))) (Math|Vector|Normalize (Math|Vector|CrossProduct (- (Transformation|GetSocketLocation (Variables|Default|GetRopeMesh) "Bone_100") (Transformation|GetActorLocation (Variables|Default|GetPlayer))) (Transformation|GetActorForwardVector (Variables|Default|GetPlayer)))))) (.yaw (Transformation|GetActorRotation (Variables|Default|GetPlayer)))) false false 0.2 false))))
      (:then_4
        ;[1 1 1] Set Player Rotation While On Rope
        (Transformation|SetWorldRotation (Variables|/Script/Engine.Character|GetCapsuleComponent (Variables|Default|GetPlayer)) (Math|Rotator|MakeRotator (.roll (Math|Rotator|MakeRotfromZY (- (Transformation|GetSocketLocation (Variables|Default|GetRopeMesh) "Bone_100") (Transformation|GetActorLocation (Variables|Default|GetPlayer))) (Math|Vector|Normalize (Math|Vector|CrossProduct (- (Transformation|GetSocketLocation (Variables|Default|GetRopeMesh) "Bone_100") (Transformation|GetActorLocation (Variables|Default|GetPlayer))) (Transformation|GetActorForwardVector (Variables|Default|GetPlayer)))))) (.pitch (Math|Rotator|MakeRotfromZY (- (Transformation|GetSocketLocation (Variables|Default|GetRopeMesh) "Bone_100") (Transformation|GetActorLocation (Variables|Default|GetPlayer))) (Math|Vector|Normalize (Math|Vector|CrossProduct (- (Transformation|GetSocketLocation (Variables|Default|GetRopeMesh) "Bone_100") (Transformation|GetActorLocation (Variables|Default|GetPlayer))) (Transformation|GetActorForwardVector (Variables|Default|GetPlayer)))))) (.yaw (Transformation|GetActorRotation (Variables|Default|GetPlayer)))) false true)))
    (else
      (Variables|Default|SetFirstVelocity (Transformation|GetVelocity (Variables|Default|GetPlayer))))))

(fn ConstructionScript
  (bind _ropemesh (Variables|Default|GetRopeMesh))
  (for _index (range 0 (- (Class|SkinnedMeshComponent|GetNumBones (Variables|Default|GetRopeMesh)) 1))
    (bind _returnvalue (AddComponent|AddBoxComponent false (Math|Transform|MakeTransform (- (Transformation|GetSocketLocation _ropemesh (Class|SkinnedMeshComponent|GetBoneName _ropemesh _index)) (Transformation|GetWorldLocation _ropemesh)) "0, 0, 0" "2.000000,2.000000,2.000000")))
    (Utilities|Array|Add (Variables|Default|GetBoneBox) _returnvalue)))

(fn FindNearestRopeBone
  (bind _ropemesh (Variables|Default|GetRopeMesh))
  (for (_array_element _array_index) (Variables|Default|GetBoneBox)
    (if (not (<= (Class|SkeletalMeshComponent|GetBoneMass _ropemesh (Class|SkinnedMeshComponent|GetBoneName _ropemesh _array_index) true) 0.0))
      (LocalVariables|SetCurrentIndex _array_index)
      (LocalVariables|SetCurrentDistance (Math|Vector|Distance(Vector) (Transformation|GetWorldLocation _array_element) (Transformation|GetSocketLocation (Variables|/Script/Engine.Character|GetMesh (Variables|Default|GetPlayer)) "head")))
      (if (or (< (LocalVariables|GetCurrentDistance) (LocalVariables|GetClosestDistance)) (< (LocalVariables|GetClosestIndex) 0))
        (LocalVariables|SetClosestIndex (LocalVariables|GetCurrentIndex))
        (LocalVariables|SetClosestDistance (LocalVariables|GetCurrentDistance)))))
  (return (LocalVariables|GetClosestIndex)))