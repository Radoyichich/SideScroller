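; BP_Switch is an interactable switch that the player character presses to toggle a list of linked objects on or off.
; Interact locks input, slides the character's capsule to the Arrow's position and rotation at its current height, then plays a push-button animation.
; After a delay it flips Status and sends ActivateMessage or DeactivateMessage to each linked object, then later restores the AnimBP and input.
; The construction script places the Arrow from PlayerTransform.
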(event EventInteract
  (params (Character :type Character%20Object%20Reference))
  (bind _arrow (Variables|Default|GetArrow))
  (bind _activatedobject (Variables|Default|GetActivatedObject))
  (bind _returnvalue (Transformation|GetWorldTransform _arrow))
  (bind _asthird_person_character (Utilities|Casting|CastToThirdPersonCharacter Character))
  (Variables|Default|SetPlayer _asthird_person_character)
  (Input|DisableInput (Variables|Default|GetPlayer) (Game|GetPlayerController 0))
  (if (not (Variables|Default|GetIsInteracting))
    (Variables|Default|SetIsInteracting true)
    (Components|MoveComponentTo (Variables|/Script/Engine.Character|GetCapsuleComponent (Variables|Default|GetPlayer)) (Math|Vector|MakeVector (.x (.location _returnvalue)) (.y (.location _returnvalue)) (.z (Transformation|GetWorldLocation (Variables|/Script/Engine.Character|GetCapsuleComponent (Variables|Default|GetPlayer))))) (.rotation _returnvalue) false false 0.2 false)
    (Components|Animation|PlayAnimation (Variables|/Script/Engine.Character|GetMesh (Variables|Default|GetPlayer)) "/Game/Character/Animations/ThirdPersonPushButton.ThirdPersonPushButton" false)
    (Utilities|FlowControl|Delay (Variables|Default|GetWaitForActivate))
    (if (== (Variables|Default|GetStatus) 0)
      (Variables|Default|SetStatus 1)
      (for _array_element _activatedobject
        (Class|BPIActivation|Activate(Message) _array_element (Variables|Default|GetPlayer)))
      (else
        (Variables|Default|SetStatus 0)
        (for _array_element_2 _activatedobject
          (Class|BPIActivation|Deactivate(Message) _array_element_2 (Variables|Default|GetPlayer)))))
    (Utilities|FlowControl|Delay (Variables|Default|GetWaitForReset))
    (Class|SkeletalMeshComponent|SetAnimClass (Variables|/Script/Engine.Character|GetMesh (Variables|Default|GetPlayer)) "/Game/Character/Animations/ThirdPerson_AnimBP.ThirdPerson_AnimBP_C")
    (Variables|Default|SetIsInteracting false)
    (Input|EnableInput (Variables|Default|GetPlayer) (Game|GetPlayerController 0))))

(fn ConstructionScript
  (Transformation|SetRelativeTransform (Variables|Default|GetArrow) (Variables|Default|GetPlayerTransform) false false))