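; BP_Door is an interactable door that slides open when activated and back when deactivated.
; Activate plays an open timeline that lerps the mesh from its current world location toward a point offset along world X, recomputed every update, so movement accumulates.
; Deactivate plays a close timeline that lerps from the current location to the position cached at BeginPlay.
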(event EventActivate
  (params (Character :type Character%20Object%20Reference))
  (bind _doormesh (Variables|Default|GetDoorMesh))
  (bind _returnvalue (Transformation|GetWorldLocation _doormesh))
  (bind (_x _y _z) (Math|Vector|BreakVector _returnvalue))
  (bind _alpha (Timeline|Open_TL PlayFromStart)
    (:Update
      (Transformation|SetWorldLocation _doormesh (Math|Vector|Lerp(Vector) _returnvalue (Math|Vector|MakeVector (- _x -2e+01) _y _z) _alpha) false false))))

(event EventDeactivate
  (params (Character :type Character%20Object%20Reference))
  (bind _doormesh (Variables|Default|GetDoorMesh))
  (bind _alpha (Timeline|Close_TL PlayFromStart)
    (:Update
      (Transformation|SetWorldLocation _doormesh (Math|Vector|Lerp(Vector) (Transformation|GetWorldLocation _doormesh) (Variables|Default|GetInitialLocation) _alpha) false false))))

(event EventBeginPlay
  (Variables|Default|SetInitialLocation (Transformation|GetWorldLocation (Variables|Default|GetDoorMesh))))

(fn ConstructionScript)