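; BP_Ladder is a climbable ladder actor, built in the construction script from a configurable count and spacing of stacked meshes plus two positioned collisions.
; Hold snaps the character in front of the ladder, facing it, stops movement and switches to Flying with climbing enabled.
; UnHold restores walking and movement-oriented rotation.
; Overlapping the top collision while climbing clears climb flags, plays a climb-up montage in Flying mode and waits out its length.
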(event OnComponentBeginOverlap(TopCollision)
  (params (OverlappedComponent :type Primitive%20Component%20Object%20Reference) (OtherActor :type Actor%20Object%20Reference) (OtherComp :type Primitive%20Component%20Object%20Reference) (OtherBodyIndex :type Integer) (bFromSweep :type Boolean) (SweepResult :type Hit%20Result%20Structure%20%28by%20ref%29))
  (bind _asthird_person_character (Utilities|Casting|CastToThirdPersonCharacter OtherActor))
  (if (Variables|/Game/Character/Character/ThirdPersonCharacter.ThirdPersonCharacter_C|GetIsClimbing _asthird_person_character)
    (Variables|/Game/Character/Character/ThirdPersonCharacter.ThirdPersonCharacter_C|SetIsClimbing _asthird_person_character false)
    (Variables|/Game/Character/Character/ThirdPersonCharacter.ThirdPersonCharacter_C|SetIsClimbingLedge _asthird_person_character false)
    (bind _returnvalue (Animation|PlayAnimMontage _asthird_person_character "/Game/Character/Animations/BracedHangToCrouch4UE4_Montage.BracedHangToCrouch4UE4_Montage" 1.0 "None"))
    (Pawn|Components|CharacterMovement|SetMovementMode (Variables|/Script/Engine.Character|GetCharacterMovement _asthird_person_character) "MOVE_Flying" 0)
    (Utilities|FlowControl|Delay _returnvalue)))

(event EventHold
  (params (Character :type Character%20Object%20Reference))
  (CallFunction|HundleInteraction Character))

(event EventUnHold
  (params (Character :type Character%20Object%20Reference))
  (bind _asthird_person_character (Utilities|Casting|CastToThirdPersonCharacter Character))
  (bind _charactermovement (Variables|/Script/Engine.Character|GetCharacterMovement _asthird_person_character))
  (Pawn|Components|CharacterMovement|SetMovementMode _charactermovement "MOVE_Walking" 0)
  (Variables|/Game/Character/Character/ThirdPersonCharacter.ThirdPersonCharacter_C|SetIsClimbing _asthird_person_character false)
  (Variables|/Script/Engine.CharacterMovementComponent|SetbOrientRotationToMovement _charactermovement true))

(fn ConstructionScript
  (for _index (range 0 (- (Variables|Default|GetLadderCount) 1))
    (bind _returnvalue (AddComponent|AddStaticMeshComponent false (Math|Transform|MakeTransform (Math|Vector|MakeVector 0.0 0.0 (* _index (Variables|Default|GetDistanceBetweenLadder))) "0, 0, 0" "1,1,1")))
    (Components|StaticMesh|SetStaticMesh _returnvalue (Variables|Default|GetLadderMesh)))
  (Transformation|SetRelativeTransform (Variables|Default|GetLadderCollision) (Variables|Default|GetLadderCollisionTransform) false false)
  (Transformation|SetRelativeTransform (Variables|Default|GetTopCollision) (Variables|Default|GetTopCollisionTransform) false false))

(fn HundleInteraction
  (params (Character :type Character%20Object%20Reference))
  (bind _returnvalue (Transformation|GetActorLocation))
  (bind _returnvalue_2 (Transformation|GetActorForwardVector))
  (bind _returnvalue_3 (Transformation|GetActorRotation))
  (bind _returnvalue_4 (* _returnvalue_2 4e+01))
  (bind _charactermovement (Variables|/Script/Engine.Character|GetCharacterMovement Character))
  (bind _returnvalue_5 (+ _returnvalue _returnvalue_4))
  (bind (_x _y) (Math|Vector|BreakVector _returnvalue_5))
  (Utilities|IsValid Character
    (:Is%20Valid
      (bind _output_get (Variables|Default|SetCharacterNewTransformLocation (Math|Transform|MakeTransform (Math|Vector|MakeVector _x _y (.Z (Math|Vector|BreakVector (Transformation|GetActorLocation Character)))) (Math|Rotator|MakeRotator (.roll _returnvalue_3) (.pitch _returnvalue_3) (+ (.yaw _returnvalue_3) 1.8e+02)) (.scale (Transformation|GetActorTransform Character)))))
      (Transformation|SetActorTransform Character _output_get)
      (Pawn|Components|CharacterMovement|SetMovementMode _charactermovement "MOVE_Flying" 0)
      (Variables|/Game/Character/Character/ThirdPersonCharacter.ThirdPersonCharacter_C|SetIsClimbing (.AsThird%20Person%20Character (Utilities|Casting|CastToThirdPersonCharacter Character)) true)
      (Variables|/Script/Engine.CharacterMovementComponent|SetbOrientRotationToMovement _charactermovement false)
      (Components|Movement|StopMovementImmediately _charactermovement))))