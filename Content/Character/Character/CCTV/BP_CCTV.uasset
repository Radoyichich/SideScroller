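; BP_CCTV is a security camera that kills the player and triggers game over when it spots them.
; Actors tagged Detectable that enter its cone arm per-tick line-of-sight checks.
; Visibility traces prioritize the player's pelvis socket while they overlap the cone, otherwise falling back to the last detected actor, which the camera mesh turns toward.
; A confirmed Player-tagged hit fires death through a DoOnce, reset when the character leaves the cone.
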(event OnComponentBeginOverlap(Cone)
  (params (OverlappedComponent :type Primitive%20Component%20Object%20Reference) (OtherActor :type Actor%20Object%20Reference) (OtherComp :type Primitive%20Component%20Object%20Reference) (OtherBodyIndex :type Integer) (bFromSweep :type Boolean) (SweepResult :type Hit%20Result%20Structure%20%28by%20ref%29))
  (if (Actor|ActorHasTag OtherActor "Detectable")
    (Variables|Default|SetDetaectedActor OtherActor)
    (Variables|Default|SetIsInArea true)))

(event OnComponentEndOverlap(Cone)
  (params (OverlappedComponent :type Primitive%20Component%20Object%20Reference) (OtherActor :type Actor%20Object%20Reference) (OtherComp :type Primitive%20Component%20Object%20Reference) (OtherBodyIndex :type Integer))
  (bind _player (Variables|Default|GetPlayer))
  (Utilities|Casting|CastToThirdPersonCharacter OtherActor)
  (Utilities|FlowControl|DoOnce false) ; enters at Reset
)

(event Custom|SetPlayerDeath
  (bind _player (Variables|Default|GetPlayer))
  (Utilities|FlowControl|DoOnce false
    (:Completed
      (Default|SetDeath _player)
      (Default|GameOver _player))))

(event EventBeginPlay
  (bind _asthird_person_character (Utilities|Casting|CastToThirdPersonCharacter (Game|GetPlayerCharacter 0)))
  (Variables|Default|SetPlayer _asthird_person_character))

(event EventTick
  (params (DeltaSeconds :type Float%20%28single-precision%29))
  (if (Variables|Default|GetIsInArea)
    (Utilities|TraceCheck
      (:True
        (Utilities|Rotate)
        (CallFunction|SetPlayerDeath))
      (:False
        (Utilities|Rotate)))))

(fn ConstructionScript)